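; Anim Notify that plays a footstep MetaSound matching the surface under the animated mesh's owner.
; On notify, it line traces on the Visibility channel from the owner's location a short distance along its negative up vector.
; The hit's physical surface type selects a Grass, Metal or Wood MetaSound, spawned at the owner's location.
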(fn ReceivedNotify
  (params (MeshComp :type Skeletal%20Mesh%20Component%20Object%20Reference) (Animation :type Anim%20Sequence%20Base%20Object%20Reference) (EventReference :type Anim%20Notify%20Event%20Reference%20Structure%20%28by%20ref%29))
  (bind _returnvalue (Components|GetOwner MeshComp))
  (bind _returnvalue_2 (Transformation|GetActorLocation _returnvalue))
  ;[0 0 0 1 90] Anim Notify BP used for playing different Footstep MetaSounds, depending on the surface type
  ; (Grass, Metal, Wood)
  (bind (_outhit _returnvalue_3) (Collision|LineTraceByChannel _returnvalue_2 (+ _returnvalue_2 (* (Transformation|GetActorUpVector _returnvalue) -2e+02)) "TraceTypeQuery1" false 0 "None"))
  (if _returnvalue_3
    (switch Utilities|FlowControl|Switch|SwitchonEPhysicalSurface (Collision|GetSurfaceType _outhit)
      (:SurfaceType1
        ;;[0.5 0.5 0.5 1 20] "MS_GrassFootstep" MetaSound
        (Audio|SpawnSoundatLocation "/Game/Audio/SFX/MS_GrassFootstep.MS_GrassFootstep" _returnvalue_2 "0, 0, 0" 1.0 1.0 0.0 "/Game/Audio/SFX/SA_Character.SA_Character" 0))
      (:SurfaceType2
        ;;[0.5 0.5 0.5 1 20] "MS_MetalFootstep" MetaSound
        (Audio|SpawnSoundatLocation "/Game/Audio/SFX/MS_MetalFootstep.MS_MetalFootstep" _returnvalue_2 "0, 0, 0" 1.0 1.0 0.0 "/Game/Audio/SFX/SA_Character.SA_Character" 0))
      (:SurfaceType3
        ;;[0.5 0.5 0.5 1 20] "MS_WoodFootstep" MetaSound
        (Audio|SpawnSoundatLocation "/Game/Audio/SFX/MS_WoodFootstep.MS_WoodFootstep" _returnvalue_2 "0, 0, 0" 1.0 1.0 0.0 "/Game/Audio/SFX/SA_Character.SA_Character" 0))))
  (return _returnvalue_3))