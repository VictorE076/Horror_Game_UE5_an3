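; One-shot checkpoint trigger that forces the first-person player's view onto the BP_Dummy actor.
; On overlap it disables the character's input and eases the control rotation toward the dummy with a short-Delay RInterpTo loop until nearly aligned.
; After a further pause it snaps the control rotation to the character's AttackTracePos rotation; input is not re-enabled here.
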(event OnComponentBeginOverlap(Checkpoint_Trigger)
  (params (OverlappedComponent :type Primitive%20Component%20Object%20Reference) (OtherActor :type Actor%20Object%20Reference) (OtherComp :type Primitive%20Component%20Object%20Reference) (OtherBodyIndex :type Integer) (bFromSweep :type Boolean) (SweepResult :type Hit%20Result%20Structure%20%28by%20ref%29))
  (bind _returnvalue (Game|GetPlayerController 0))
  (bind _returnvalue_2 (Pawn|GetControlRotation _returnvalue :!class /Script/Engine.Controller))
  (if (not (Variables|CheckpointTrigger|GetPlayer%20already%20looked%20at%20Dummy?))
    (bind _asbp_true_first_person_character (Utilities|Casting|CastToBP_TrueFirstPersonCharacter OtherActor))
    (bind _returnvalue_3 (Actor|GetActorOfClass "/Game/Dummy/Blueprints/BP_Dummy.BP_Dummy_C"))
    (Utilities|IsValid _returnvalue_3
      (:Is%20Valid
        (Variables|CheckpointTrigger|SetPlayer%20already%20looked%20at%20Dummy? true)
        (Input|DisableInput _asbp_true_first_person_character 0) ; Player will not be able to move anymore\n(stack of input handled by a PlayerController)
        ;[0.4 0.3 0.6 0.2 30] LOOK AT Dummy -> Rotating the player's CAMERA towards the EnemyAI (in a LOOP).
        (if (Utilities|Operators|NotEqual(!=) _returnvalue_2 (Math|Rotator|FindLookatRotation (Transformation|GetActorLocation _asbp_true_first_person_character) (Transformation|GetActorLocation _returnvalue_3)) 1.0) :!label _label
          (Utilities|FlowControl|Delay 0.001) ; "0.001" seconds Delay\n(Used to prevent INFINITE LOOP)
          (Pawn|SetControlRotation (Game|GetPlayerController 0) (Math|Interpolation|RInterpTo _returnvalue_2 (Math|Rotator|FindLookatRotation (Transformation|GetActorLocation _asbp_true_first_person_character) (Transformation|GetActorLocation _returnvalue_3)) (Utilities|Time|GetWorldDeltaSeconds) 1.5)) ; Rotating the player's CAMERA\ntowards the EnemyAI
          (goto _label)
          (else
            (bind _asbp_true_first_person_character_2 (Utilities|Casting|CastToBP_TrueFirstPersonCharacter (Game|GetPlayerCharacter 0)))
            (Utilities|FlowControl|Delay 1e+01)
            (Pawn|SetControlRotation (Game|GetPlayerController 0) (Transformation|GetWorldRotation (Variables|/Game/ThirdPerson/Blueprints/BP_TrueFirstPersonCharacter.BP_TrueFirstPersonCharacter_C|GetAttack%20Trace%20Pos _asbp_true_first_person_character_2))) ; Rotating the player's CAMERA\ntowards the EnemyAI
          ))))))

(event EventBeginPlay)

(event Collision|EventActorBeginOverlap
  (params (OtherActor :type Actor%20Object%20Reference)))

(event EventTick
  (params (DeltaSeconds :type Float%20%28single-precision%29)))

(fn ConstructionScript)