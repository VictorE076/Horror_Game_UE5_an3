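; BP_Dummy is a dummy actor that repeatedly screams for help through a positional audio component.
; BeginPlay starts a custom event that, after a short delay, uses a random MultiGate to pick one of two help clips and store its duration.
; It plays the clip, prints "HELP" on screen, waits for that duration plus a random pause, then resets and re-enters the MultiGate to loop with natural-sounding spacing.
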(event Custom|Help%20Dummy%20Sound%20System
  ;[0.25 0.5 0 0.2 50] After an initial DELAY of "3.0" seconds, it sets (in a LOOP with a specified DELAY at the end) a Random "Help_Dummy" 3D Sound to Play at its location.
  (Utilities|FlowControl|Delay 3.0) ; "3.0" seconds Delay
  (Utilities|FlowControl|MultiGate true false -1 :!label _label ; Executes a series of pins,\nrandomly ("Is Random" = TRUE)
    (:Out%200
      (Audio|Components|Audio|SetSound (Variables|Default|GetAudio_Help) "/Game/Audio/SFX/Help_Dummy.Help_Dummy") ; "Help_Dummy" 3D Sound\n("SA_Help_Dummy" Sound Attenuation)
      (Variables|Default|SetAudio%20Help%20Dummy%20Duration 3.42))
    (:Out%201
      (Audio|Components|Audio|SetSound (Variables|Default|GetAudio_Help) "/Game/Audio/SFX/Help_please_Dummy.Help_please_Dummy") ; "Help_please_Dummy" 3D Sound\n("SA_Help_Dummy" Sound Attenuation)
      (Variables|Default|SetAudio%20Help%20Dummy%20Duration 1.31)))
  (Audio|Components|Audio|Play (Variables|Default|GetAudio_Help) 0.0) ; Play "Audio_Help" 3D Sound,\nimmediately
  (Development|PrintString "HELP" true true "(R=1.000000,G=0.250000,B=0.000000,A=1.000000)" 5.0)
  ;;[0.5 0.5 0.5 1 29] DELAY
  ;; ("Help_Dummy" Sound Duration + Random Float in Range).
  (Utilities|FlowControl|Delay (+ (Variables|Default|GetAudio%20Help%20Dummy%20Duration) (Math|Random|RandomFloatinRange 2.0 4.0)))
  (CallFunction|ResetHelpDummySoundsMULTIGATE) ; Custom Event to reset the previous MULTIGATE
  (goto _label))

(event Custom|Reset%20Help%20Dummy%20Sounds%20MULTIGATE
  ;[0.25 0.5 0 0.2 50] After an initial DELAY of "3.0" seconds, it sets (in a LOOP with a specified DELAY at the end) a Random "Help_Dummy" 3D Sound to Play at its location.
  (Utilities|FlowControl|MultiGate true false -1) ; enters at Reset
)

(event EventBeginPlay
  ;[1 0.25 0 0.2 40] Creating and executing the "Help Dummy Sound System" for managing Dummy's HELP Screams in a more natural way, in game.
  (CallFunction|HelpDummySoundSystem) ; Custom Event
)

(event Collision|EventActorBeginOverlap
  (params (OtherActor :type Actor%20Object%20Reference)))

(event EventTick
  (params (DeltaSeconds :type Float%20%28single-precision%29)))

(fn ConstructionScript)