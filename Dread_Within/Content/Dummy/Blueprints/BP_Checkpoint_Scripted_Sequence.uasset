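; One-shot trigger actor that runs the third-mission horror cutscene when the player overlaps it while a Dummy exists.
; It locks input, eases the camera toward the Dummy through a looping delayed RInterpTo macro, then swaps it behind a black screen for a jumpscare Horror Dummy.
; Delays time the sounds, screens and flashlight dimming.
; Afterward it makes the flashlight flicker, restores HUD and input, issues the next objective and spawns a portal.
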(event OnComponentBeginOverlap(Checkpoint_Trigger)
  (params (OverlappedComponent :type Primitive%20Component%20Object%20Reference) (OtherActor :type Actor%20Object%20Reference) (OtherComp :type Primitive%20Component%20Object%20Reference) (OtherBodyIndex :type Integer) (bFromSweep :type Boolean) (SweepResult :type Hit%20Result%20Structure%20%28by%20ref%29))
  ;[0.1 0 0.1 0.2 120] "Checkpoint_Scripted_Sequence" (Player can trigger it just ONCE, on the 3-rd mission).
  (if (not (Variables|CheckpointTrigger|GetPlayer%20already%20looked%20at%20Dummy?))
    (bind _asbp_true_first_person_character (Utilities|Casting|CastToBP_TrueFirstPersonCharacter OtherActor))
    (bind _returnvalue (Actor|GetActorOfClass "/Game/Dummy/Blueprints/BP_Dummy.BP_Dummy_C"))
    (Utilities|IsValid _returnvalue
      (:Is%20Valid
        (Variables|CheckpointTrigger|SetPlayer%20already%20looked%20at%20Dummy? true)
        (Variables|Dummy|SetTemp%20Location%20Dummy (Transformation|GetActorLocation _returnvalue))
        ;;[0.2 0.2 0.2 1 40] Removes the "WB_Health_Stamina" Widget owned only by this Player, from its parent.
        (Widget|RemovefromParent (Variables|/Game/ThirdPerson/Blueprints/BP_TrueFirstPersonCharacter.BP_TrueFirstPersonCharacter_C|GetWB_Health_Stamina _asbp_true_first_person_character))
        (Development|PrintString "HEALTH_STAMINA REMOVED" true true "(R=0.500000,G=0.000000,B=1.000000,A=1.000000)" 3.0)
        ;;[0.5 0.5 0.5 1 30] Disable Input (for the player)
        (Input|DisableInput _asbp_true_first_person_character 0) ; Player will not be able to move anymore\n(stack of input handled by a PlayerController)
        ;;[0.4 0.3 0.6 0.2 30] LOOK AT Dummy
        (Utilities|LOOKATDUMMY
          (:Out%20Exec
            ;;[0.5 0.5 0.5 1 30] If Valid, "Player Gasping For Air" 2D Sound will "Fade Out" for "1.0" second, until stopping completely.
            (bind _asbp_true_first_person_character_2 (Utilities|Casting|CastToBP_TrueFirstPersonCharacter (Game|GetPlayerCharacter 0)))
            (Utilities|IsValid (Variables|/Game/ThirdPerson/Blueprints/BP_TrueFirstPersonCharacter.BP_TrueFirstPersonCharacter_C|GetPlayer_gasping_for_air _asbp_true_first_person_character_2)
              (:Is%20Valid
                (Audio|Components|Audio|FadeOut (Variables|/Game/ThirdPerson/Blueprints/BP_TrueFirstPersonCharacter.BP_TrueFirstPersonCharacter_C|GetPlayer_gasping_for_air _asbp_true_first_person_character_2) 0.5 0.0 "Linear" :!class /Script/Engine.AudioComponent))
              (:Is%20Not%20Valid
                _))
            (Development|PrintString "NO SOUND" true true "(R=1.000000,G=0.500000,B=0.000000,A=1.000000)" 3.0)
            ;;[0.5 0.5 0.5 1 30] Player screaming " I'LL SAVE YOU" to Dummy.
            (Audio|PlaySound2D "/Game/Audio/SFX/ElevenLabs_Liam__I_WILL_SAVE_YOU__.ElevenLabs_Liam__I_WILL_SAVE_YOU__" 1.0 1.0 0.0 0 0) ; "ElevenLabs_Liam_I_WILL_SAVE_YOU__" 2D Sound
            (Development|PrintString "SAVE YOU" true true "(R=1.000000,G=1.000000,B=0.000000,A=1.000000)" 3.0)
            (Utilities|FlowControl|Delay 2.5) ; "2.5" seconds Delay
            ;;[0 0 0 1 60] BLACK SCREEN
            ;;;[0.2 0.2 0.2 1 40] Creates the "WB_BlackScreen" Widget owned only by this Player, then adds the Widget to Viewport
            (bind _returnvalue_2 (UserInterface|CreateWidget "/Game/UI/WB_BlackScreen.WB_BlackScreen_C" (Game|GetPlayerController 0)))
            (bind _output_get (Variables|WBBlackScreen|SetWB%20BlackScreen _returnvalue_2))
            (UserInterface|Viewport|AddtoViewport _output_get 10 :!pinned true) ; ZOrder = 10
            (Development|PrintString "BLACK SCREEN " true true "(R=0.500000,G=0.000000,B=1.000000,A=1.000000)" 3.0)
            (Utilities|FlowControl|Delay 0.2) ; "0.2" seconds Delay
            ;;;[0.5 0.5 0.5 1 30] "Destroy BP_Dummy" Custom Event
            (CallFunction|DestroyBPDummy)
            (Development|PrintString "Destroy Dummy" true true "(R=1.000000,G=0.100000,B=0.000000,A=1.000000)" 3.0)
            (Utilities|FlowControl|Delay 0.5) ; "0.5" seconds Delay
            ;;;[0.5 0.5 0.5 1 30] Player's Camera will be parallel to the ground ("Horror Dummy Trace Pos" Arrow Orientation).
            (bind _asbp_true_first_person_character_3 (Utilities|Casting|CastToBP_TrueFirstPersonCharacter (Game|GetPlayerCharacter 0)))
            (Pawn|SetControlRotation (Game|GetPlayerController 0) (Transformation|GetWorldRotation (Variables|/Game/ThirdPerson/Blueprints/BP_TrueFirstPersonCharacter.BP_TrueFirstPersonCharacter_C|GetHorror_Dummy%20Trace%20Pos _asbp_true_first_person_character_3))) ; Rotating the player's CAMERA\ntowards the EnemyAI
            (Development|PrintString "Camera" true true "(R=0.000000,G=0.200000,B=0.800000,A=1.000000)" 3.0)
            (Utilities|FlowControl|Delay 0.5) ; "0.5" seconds Delay
            ;;;[0.5 0.5 0.5 1 30] "Scared Breath Loop" 2D Sound will "Play" for "5.0" seconds, then it will "Stop".
            (bind _asbp_true_first_person_character_4 (Utilities|Casting|CastToBP_TrueFirstPersonCharacter (Game|GetPlayerCharacter 0)))
            (Utilities|IsValid (Variables|/Game/ThirdPerson/Blueprints/BP_TrueFirstPersonCharacter.BP_TrueFirstPersonCharacter_C|GetScaredBreathLoop _asbp_true_first_person_character_4)
              (:Is%20Valid
                (Audio|Components|Audio|Stop (Variables|/Game/ThirdPerson/Blueprints/BP_TrueFirstPersonCharacter.BP_TrueFirstPersonCharacter_C|GetScaredBreathLoop _asbp_true_first_person_character_4)))
              (:Is%20Not%20Valid
                _))
            (bind _returnvalue_3 (Audio|SpawnSound2D "/Game/Audio/SFX/Scared_breath_loop.Scared_breath_loop" 1.0 1.0 0.0 0)) ; Spawning "Scared_breath_Loop" 2D Sound
            (bind _output_get_2 (Variables|/Game/ThirdPerson/Blueprints/BP_TrueFirstPersonCharacter.BP_TrueFirstPersonCharacter_C|SetScaredBreathLoop _asbp_true_first_person_character_4 _returnvalue_3))
            (Audio|Components|Audio|StopDelayed _output_get_2 5.0) ; "5.0" seconds Delayed Stop
            (Development|PrintString "Breath" true true "(R=0.200000,G=0.700000,B=1.000000,A=1.000000)" 3.0)
            ;;;[0.5 0.5 0.5 1 30] Spawning "Horror_Dummy" Character in front of the player.
            (bind _asbp_true_first_person_character_5 (Utilities|Casting|CastToBP_TrueFirstPersonCharacter (Game|GetPlayerCharacter 0)))
            (Game|SpawnActorfromClass "/Game/Dummy/Horror_Dummy/Blueprints/BP_Horror_Dummy.BP_Horror_Dummy_C" (Math|Transform|MakeTransform (+ (Transformation|GetWorldLocation (Variables|/Game/ThirdPerson/Blueprints/BP_TrueFirstPersonCharacter.BP_TrueFirstPersonCharacter_C|GetHorror_Dummy%20Trace%20Pos _asbp_true_first_person_character_5)) (* (Math|Vector|GetForwardVector (Transformation|GetWorldRotation (Variables|/Game/ThirdPerson/Blueprints/BP_TrueFirstPersonCharacter.BP_TrueFirstPersonCharacter_C|GetHorror_Dummy%20Trace%20Pos _asbp_true_first_person_character_5))) (Math|Float|MakeLiteralFloat 5e+01))) (Math|Rotator|MakeRotator 0.0 0.0 (.yaw (Math|Rotator|FindLookatRotation (+ (Transformation|GetWorldLocation (Variables|/Game/ThirdPerson/Blueprints/BP_TrueFirstPersonCharacter.BP_TrueFirstPersonCharacter_C|GetHorror_Dummy%20Trace%20Pos _asbp_true_first_person_character_5)) (* (Math|Vector|GetForwardVector (Transformation|GetWorldRotation (Variables|/Game/ThirdPerson/Blueprints/BP_TrueFirstPersonCharacter.BP_TrueFirstPersonCharacter_C|GetHorror_Dummy%20Trace%20Pos _asbp_true_first_person_character_5))) (Math|Float|MakeLiteralFloat 5e+01))) (Transformation|GetActorLocation _asbp_true_first_person_character_5)))) "1.000000,1.000000,1.000000") "AlwaysSpawn" "MultiplyWithRoot" 0 _asbp_true_first_person_character_5) ; Always Spawns the "Horror_Dummy" Actor with the calculated "Transform [Location, Rotation (0, 0, Z), Scale]",\n"Ignoring Collisions" and using the "Multiply Scale With Root Component Scale".\nPlayer is the "Instigator" Pawn responsible for other gameplay events caused by "BP_Checkpoint_Dummy" Actor.
            (Development|PrintString "SPAWNED" true true "(R=0.000000,G=0.500000,B=1.000000,A=1.000000)" 3.0)
            ;;;[0.5 0.5 0.5 1 30] Turning ON Player's flashlight having a much smaller "intensity" (effect used so player can see much better, the "Horror_Dummy" in from of him).
            (bind _asbp_true_first_person_character_6 (Utilities|Casting|CastToBP_TrueFirstPersonCharacter (Game|GetPlayerCharacter 0)))
            (Default|TurnONFlashlight _asbp_true_first_person_character_6)
            (Rendering|Components|Light|SetIntensity (Variables|/Game/ThirdPerson/Blueprints/BP_TrueFirstPersonCharacter.BP_TrueFirstPersonCharacter_C|GetFlashlight _asbp_true_first_person_character_6) (* (Variables|/Script/Engine.LightComponentBase|GetIntensity (Variables|/Game/ThirdPerson/Blueprints/BP_TrueFirstPersonCharacter.BP_TrueFirstPersonCharacter_C|GetFlashlight _asbp_true_first_person_character_6)) 0.04))
            (Development|PrintString (Utilities|String|ToString(Float) (Variables|/Script/Engine.LightComponentBase|GetIntensity (Variables|/Game/ThirdPerson/Blueprints/BP_TrueFirstPersonCharacter.BP_TrueFirstPersonCharacter_C|GetFlashlight _asbp_true_first_person_character_6))) true true "(R=0.800000,G=0.800000,B=0.800000,A=1.000000)" 3e+01)
            (Utilities|FlowControl|Delay 5.0) ; "5.0" seconds Delay
            ;;;[0.2 0.2 0.2 1 40] Removes the "WB_BlackScreen" Widget owned only by this Player, from its parent.
            (Widget|RemovefromParent (Variables|WBBlackScreen|GetWB%20BlackScreen))
            (Development|PrintString "BLACK SCREEN REMOVED" true true "(R=0.500000,G=0.000000,B=1.000000,A=1.000000)" 3.0)
            ;;[0.5 0.5 0.5 1 30] Player scared by "Horror_Dummy" ( + "JumpscareEvil" 2D Sound )
            (Audio|PlaySound2D "/Game/Audio/SFX/JumpscareEvil.JumpscareEvil" 1.0 1.0 0.0 0 0) ; "JumpscareEvil" 2D Sound
            (Utilities|FlowControl|Delay 0.1) ; "0.1" seconds Delay
            (Audio|PlaySound2D "/Game/Audio/SFX/Scream_fear.Scream_fear" 1.0 1.0 0.0 0 0) ; "Scream_fear" 2D Sound
            (Utilities|FlowControl|Delay 1.1) ; "1.1" seconds Delay
            (bind _asbp_true_first_person_character_7 (Utilities|Casting|CastToBP_TrueFirstPersonCharacter (Game|GetPlayerCharacter 0)))
            (bind _returnvalue_4 (Audio|SpawnSound2D "/Game/Audio/SFX/Player_gasping_for_air.Player_gasping_for_air" 1.0 1.0 0.0 0)) ; Spawning "Player_gasping_for_air" 2D Sound
            (Variables|/Game/ThirdPerson/Blueprints/BP_TrueFirstPersonCharacter.BP_TrueFirstPersonCharacter_C|SetPlayer_gasping_for_air _asbp_true_first_person_character_7 _returnvalue_4)
            (Development|PrintString "Player SCARED" true true "(R=0.500000,G=0.000000,B=0.800000,A=1.000000)" 3.0)
            (Utilities|FlowControl|Delay 4.0) ; "4.0" seconds Delay
            ;;[0 0 0 1 60] BLACK SCREEN (again)
            ;;;[0.2 0.2 0.2 1 40] Creates (again) the "WB_BlackScreen" Widget owned only by this Player, then adds the Widget to Viewport
            (bind _returnvalue_5 (UserInterface|CreateWidget "/Game/UI/WB_BlackScreen.WB_BlackScreen_C" (Game|GetPlayerController 0)))
            (bind _output_get_3 (Variables|WBBlackScreen|SetWB%20BlackScreen _returnvalue_5))
            (UserInterface|Viewport|AddtoViewport _output_get_3 10 :!pinned true) ; ZOrder = 10
            (Development|PrintString "BLACK SCREEN " true true "(R=0.500000,G=0.000000,B=1.000000,A=1.000000)" 3.0)
            (Utilities|FlowControl|Delay 1.2) ; "1.2" seconds Delay
            ;;;[0.5 0.5 0.5 1 30] "Breath_stinger" 2D Sound caused by Horror Dummy.
            (Audio|PlaySound2D "/Game/Audio/SFX/Breath_stinger.Breath_stinger" 1.0 1.0 0.0 0 0) ; "Breath_stinger" 2D Sound
            (Development|PrintString "Breath Stinger " true true "(R=0.500000,G=1.000000,B=1.000000,A=1.000000)" 3.0)
            ;;;[0.5 0.5 0.5 1 30] Destroying Horror Dummy Character if existing on the map.
            (bind _returnvalue_6 (Actor|GetActorOfClass "/Game/Dummy/Horror_Dummy/Blueprints/BP_Horror_Dummy.BP_Horror_Dummy_C"))
            (Utilities|IsValid _returnvalue_6
              (:Is%20Valid
                (Actor|DestroyActor _returnvalue_6)
                (Development|PrintString "Destroy Horror Dummy" true true "(R=1.000000,G=0.100000,B=0.000000,A=1.000000)" 3.0)
                ;;;[0.5 0.5 0.5 1 30] Player's flashlight will regain its normal "intensity".
                (bind _asbp_true_first_person_character_8 (Utilities|Casting|CastToBP_TrueFirstPersonCharacter (Game|GetPlayerCharacter 0)))
                (Rendering|Components|Light|SetIntensity (Variables|/Game/ThirdPerson/Blueprints/BP_TrueFirstPersonCharacter.BP_TrueFirstPersonCharacter_C|GetFlashlight _asbp_true_first_person_character_8) (* (Variables|/Script/Engine.LightComponentBase|GetIntensity (Variables|/Game/ThirdPerson/Blueprints/BP_TrueFirstPersonCharacter.BP_TrueFirstPersonCharacter_C|GetFlashlight _asbp_true_first_person_character_8)) 25.0))
                (Development|PrintString (Utilities|String|ToString(Float) (Variables|/Script/Engine.LightComponentBase|GetIntensity (Variables|/Game/ThirdPerson/Blueprints/BP_TrueFirstPersonCharacter.BP_TrueFirstPersonCharacter_C|GetFlashlight _asbp_true_first_person_character_8))) true true "(R=0.200000,G=0.200000,B=0.200000,A=1.000000)" 2e+01)
                ;;;[0.4 0.3 0.6 0.2 30] LOOK AT Dummy
                (Utilities|LOOKATDUMMY
                  (:Out%20Exec
                    ;;;[0.8 0.8 0.8 1 30] Making the player's flashlight flicker.
                    (CallFunction|FlickeringFlashlight)
                    (Development|PrintString "Flickering Flashlight" true true "(R=0.500000,G=0.500000,B=0.500000,A=1.000000)" 3.0)
                    (Utilities|FlowControl|Delay 0.5) ; "0.5" seconds Delay
                    ;;;[0.2 0.2 0.2 1 40] Removes (again) the "WB_BlackScreen" Widget owned only by this Player, from its parent.
                    (Widget|RemovefromParent (Variables|WBBlackScreen|GetWB%20BlackScreen))
                    (Development|PrintString "BLACK SCREEN REMOVED" true true "(R=0.500000,G=0.000000,B=1.000000,A=1.000000)" 3.0)
                    (Utilities|FlowControl|Delay 2.0) ; "2.0" seconds Delay
                    ;;[0.2 0.2 0.2 1 40] Creates (again) the "WB_Health_Stamina" Widget owned only by this Player, then adds the Widget to Viewport
                    (bind _asbp_true_first_person_character_9 (Utilities|Casting|CastToBP_TrueFirstPersonCharacter (Game|GetPlayerCharacter 0)))
                    (bind _returnvalue_7 (UserInterface|CreateWidget "/Game/UI/WB_Health_Stamina.WB_Health_Stamina_C" (Game|GetPlayerController 0)))
                    (bind _output_get_4 (Variables|/Game/ThirdPerson/Blueprints/BP_TrueFirstPersonCharacter.BP_TrueFirstPersonCharacter_C|SetWB_Health_Stamina _asbp_true_first_person_character_9 _returnvalue_7))
                    (UserInterface|Viewport|AddtoViewport _output_get_4 -10 :!pinned true) ; ZOrder = -10
                    (Development|PrintString "HEALTH_STAMINA" true true "(R=0.500000,G=0.000000,B=1.000000,A=1.000000)" 3.0)
                    ;;[0.5 0.5 0.5 1 30] Enable Input (for the player)
                    (bind _asbp_true_first_person_character_10 (Utilities|Casting|CastToBP_TrueFirstPersonCharacter (Game|GetPlayerCharacter 0)))
                    (Input|EnableInput _asbp_true_first_person_character_10 0) ; Player will be able to move again\n(stack of input handled by a PlayerController)
                    (Development|PrintString "Enable Input" true true "(R=0.000000,G=0.700000,B=0.000000,A=1.000000)" 3.0)
                    ;;[1 0.25 0.75 0.2 40] NEW Objective (4-th).
                    (bind _asbp_true_first_person_character_11 (Utilities|Casting|CastToBP_TrueFirstPersonCharacter (Game|GetPlayerCharacter 0)))
                    (Default|NEWObjective _asbp_true_first_person_character_11 3) ; New Objective Notification
                    ;;[0 0.5 0.5 0.2 40] Spawning the "Portal" Actor ("BP_Portal") in the World at the corresponding Location.
                    (CallFunction|SpawnPortal)
                    (Development|PrintString "Portal" true true "(R=0.000000,G=0.500000,B=1.000000,A=1.000000)" 3.0)
                    ;;[0.5 0.5 0.5 1 30] "Scared Breath Loop" 2D Sound will "Play" for "5.0" seconds, then it will "Fade Out" for "2.0" seconds (2D Sound played just ONCE).
                    (bind _asbp_true_first_person_character_12 (Utilities|Casting|CastToBP_TrueFirstPersonCharacter (Game|GetPlayerCharacter 0)))
                    (Utilities|IsValid (Variables|/Game/ThirdPerson/Blueprints/BP_TrueFirstPersonCharacter.BP_TrueFirstPersonCharacter_C|GetScaredBreathLoop _asbp_true_first_person_character_12)
                      (:Is%20Valid
                        (Audio|Components|Audio|Stop (Variables|/Game/ThirdPerson/Blueprints/BP_TrueFirstPersonCharacter.BP_TrueFirstPersonCharacter_C|GetScaredBreathLoop _asbp_true_first_person_character_12)))
                      (:Is%20Not%20Valid
                        _))
                    (bind _returnvalue_8 (Audio|SpawnSound2D "/Game/Audio/SFX/Scared_breath_loop.Scared_breath_loop" 1.0 1.0 0.0 0)) ; Spawning "Scared_breath_Loop" 2D Sound
                    (bind _output_get_5 (Variables|/Game/ThirdPerson/Blueprints/BP_TrueFirstPersonCharacter.BP_TrueFirstPersonCharacter_C|SetScaredBreathLoop _asbp_true_first_person_character_12 _returnvalue_8))
                    (Utilities|FlowControl|Delay 5.0) ; "5.0" seconds Delay
                    (Audio|Components|Audio|FadeOut _output_get_5 2.0 0.0 "Linear" :!class /Script/Engine.AudioComponent)
                    (Development|PrintString "Breath" true true "(R=0.200000,G=0.700000,B=1.000000,A=1.000000)" 3.0)))))))))))

(event Custom|Destroy%20BP_Dummy
  ;[0.5 0.5 0.5 1 30] Destroying Dummy Character if existing on the map.
  (bind _returnvalue (Actor|GetActorOfClass "/Game/Dummy/Blueprints/BP_Dummy.BP_Dummy_C"))
  (Utilities|IsValid _returnvalue
    (:Is%20Valid
      (Actor|DestroyActor _returnvalue))))

(event Custom|Spawn%20Portal
  ;[0 0.5 0.5 0.2 40] Spawning the "Portal" Actor ("BP_Portal") in the World with the corresponding "Location" Coordinates [ (9910, 18330, 1340) ], "Ignoring Collisions", Player being the "Instigator" Pawn.
  (bind _asbp_true_first_person_character (Utilities|Casting|CastToBP_TrueFirstPersonCharacter (Game|GetPlayerCharacter 0)))
  (Game|SpawnActorfromClass "/Game/Blueprints/BP_Portal.BP_Portal_C" (Math|Transform|MakeTransform "9910.000000,18330.000000,1340.000000" "0, 0, 0" "1.000000,1.000000,1.000000") "AlwaysSpawn" "MultiplyWithRoot" 0 _asbp_true_first_person_character) ; Always Spawns the "Portal" Actor with the specified "Transform (Location, Rotation, Scale)",\n"Ignoring Collisions" and using the "Multiply Scale With Root Component Scale".\nPlayer is the "Instigator" Pawn responsible for damage and other gameplay events caused by "BP_Portal" Actor.
)

(event Custom|Flickering%20Flashlight
  ;[0.8 0.8 0.8 1 30] Making the player's flashlight flicker
  ; -> "Low" Graphics will keep Shadow Quality to "Medium".
  (bind _asbp_true_first_person_character (Utilities|Casting|CastToBP_TrueFirstPersonCharacter (Game|GetPlayerCharacter 0)))
  (Rendering|Components|Light|SetLightFunctionMaterial (Variables|/Game/ThirdPerson/Blueprints/BP_TrueFirstPersonCharacter.BP_TrueFirstPersonCharacter_C|GetFlashlight _asbp_true_first_person_character) "/Game/Materials/MyMaterials/Light_Flicker_Material.Light_Flicker_Material")
  (bind _returnvalue (Settings|GetGameUserSettings)) ; Returns the game local machine settings\n(resolution, windowing mode, etc.)
  (Class|GameUserSettings|SetShadowQuality _returnvalue (Math|Integer|Clamp(Integer) (Class|GameUserSettings|GetOverallScalabilityLevel _returnvalue) 1 4)) ; Sets the "Shadow" Quality to the "Overall Scalability Level"\nvalue 'clamped' to be between '1' and '4' (inclusive)
  (Class|GameUserSettings|ApplySettings _returnvalue true) ; Applies all current User Settings to the game\nand Saves to "permanent storage" (e.g. file),\noptionally checking for command line overrides.
)

(event EventBeginPlay)

(event Collision|EventActorBeginOverlap
  (params (OtherActor :type Actor%20Object%20Reference)))

(event EventTick
  (params (DeltaSeconds :type Float%20%28single-precision%29)))

(fn ConstructionScript)