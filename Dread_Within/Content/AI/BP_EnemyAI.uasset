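; Zombie enemy character that chases and attacks the player, and whose death advances the objective and spawns a portal.
; Pawn sensing sets a blackboard chase flag and fades in chase music; a looping one-second timer clears both.
; AttackPlayer plays a given montage and sphere-traces to apply damage.
; Taking damage triggers a hit indicator and stun reaction, or at zero health ragdolls the enemy and stops its behavior tree.
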(event OnSeePawn(PawnSensing)
  (params (Pawn :type Pawn%20Object%20Reference))
  ;[0 1 0 0.2 50] Events triggered when the EnemyAI sees or hears a Pawn (the Player in this case) -> All based on "Pawn Sensing Component" AI configuration values
  ; These two Events do nothing if the EnemyAI is already STUNNED or DEAD.
  (if (and (Actor|ActorHasTag Pawn "Player") (and (not (Variables|Default|GetEnemyAI%20stunned?)) (not (Variables|Default|GetEnemyAI%20dead?))))
    ;;[0.4896 0.4896 0.4896 1 30] "seeing_or_hearingPlayer?" is a bool variable/key in the "BD_AI" and we'll set it to TRUE
    (AI|Components|Blackboard|SetValueasBool (AI|GetBlackboard (AI|GetAIController self)) (Utilities|Name|MakeLiteralName "seeing_or_hearingPlayer?") true)
    ;[0 0.25 1 0.2 50] When EnemyAI sees or hears a Pawn (the Player in this case), "Chasing_Violins_Loop" Sound will Spawn and then "Fade In" (2 seconds Duration), if "ChasingSoundLoop" Audio Component is NOT Playing at this moment, otherwise if the Player is already "dead", then "Chasing_Violins_Loop" Sound will "Fade Out" (2 seconds Duration)
    (if (not (Utilities|IsValid (Variables|Default|GetChasingSoundLoop)))
      (bind _returnvalue (Audio|SpawnSound2D "/Game/Audio/SFX/Chasing_Violins_Loop.Chasing_Violins_Loop" 2.0 1.0 0.0 0)) ; This allows users to create "Audio Components" Variables.\nSound instances will begin playing upon this "Audio Component" (2 * volume)
      ;;[0.3594 0.3594 0.3594 1 30] "ChasingSoundLoop" Audio Component will Play louder and louder (Linear Fade Curve) over 2 seconds, until reaching the "Volume Multiplier" Value (2 * Volume).
      (bind _output_get (Variables|Default|SetChasingSoundLoop _returnvalue))
      (Audio|Components|Audio|FadeIn _output_get 2.0 1.0 0.0 "Linear" :!class /Script/Engine.AudioComponent) ; This allows designers to call "Play" on an "Audio Component Instance" (ChasingSoundLoop) while applying a "Volume Curve" (Linear) over a certain time (2 seconds).\nParameters allow designers to indicate the duration of the "Fade" (2 seconds), the "Curve Shape" and the "Start Time" if seeking into the sound.
      (else
        (bind _player_dead_ (CallFunction|IsPlayerDead)) ; Function which checks if the Player is already "dead"!
        (if _player_dead_
          ;;[0.5052 0.5052 0.5052 1 30] "ChasingSoundLoop" Audio Component will Play softer and softer (Linear Fade Curve) over 2 seconds, until stopping completely.
          (Audio|Components|Audio|FadeOut (Variables|Default|GetChasingSoundLoop) 2.0 0.0 "Linear" :!class /Script/Engine.AudioComponent) ; This allows designers to call "Play" on an "Audio Component Instance" (ChasingSoundLoop) while applying a "Volume Curve" (Linear) over a certain time (2 seconds).\nParameters allow designers to indicate the duration of the "Fade" (2 seconds), the "Curve Shape" and the "Start Time" if seeking into the sound.
        )))))

(event OnHearNoise(PawnSensing)
  (params (Instigator :type Pawn%20Object%20Reference) (Location :type Vector%20%28by%20ref%29 :default "0, 0, 0") (Volume :type Float%20%28single-precision%29))
  ;[0 1 0 0.2 50] Events triggered when the EnemyAI sees or hears a Pawn (the Player in this case) -> All based on "Pawn Sensing Component" AI configuration values
  ; These two Events do nothing if the EnemyAI is already STUNNED or DEAD.
  ;;[0.4948 0.4948 0.4948 1 25] A single sound made by the Player will be percepted by the EnemyAI for 3 seconds (See "PawnSensing" -> Hearing Max Sound Age)
  (if (and (Actor|ActorHasTag Instigator "Player") (and (not (Variables|Default|GetEnemyAI%20stunned?)) (not (Variables|Default|GetEnemyAI%20dead?))))
    ;;[0.4896 0.4896 0.4896 1 30] "seeing_or_hearingPlayer?" is a bool variable/key in the "BD_AI" and we'll set it to TRUE
    (AI|Components|Blackboard|SetValueasBool (AI|GetBlackboard (AI|GetAIController self)) (Utilities|Name|MakeLiteralName "seeing_or_hearingPlayer?") true)
    ;[0 0.25 1 0.2 50] When EnemyAI sees or hears a Pawn (the Player in this case), "Chasing_Violins_Loop" Sound will Spawn and then "Fade In" (2 seconds Duration), if "ChasingSoundLoop" Audio Component is NOT Playing at this moment, otherwise if the Player is already "dead", then "Chasing_Violins_Loop" Sound will "Fade Out" (2 seconds Duration)
    (if (not (Utilities|IsValid (Variables|Default|GetChasingSoundLoop)))
      (bind _returnvalue (Audio|SpawnSound2D "/Game/Audio/SFX/Chasing_Violins_Loop.Chasing_Violins_Loop" 2.0 1.0 0.0 0)) ; This allows users to create "Audio Components" Variables.\nSound instances will begin playing upon this "Audio Component" (2 * volume)
      ;;[0.3594 0.3594 0.3594 1 30] "ChasingSoundLoop" Audio Component will Play louder and louder (Linear Fade Curve) over 2 seconds, until reaching the "Volume Multiplier" Value (2 * Volume).
      (bind _output_get (Variables|Default|SetChasingSoundLoop _returnvalue))
      (Audio|Components|Audio|FadeIn _output_get 2.0 1.0 0.0 "Linear" :!class /Script/Engine.AudioComponent) ; This allows designers to call "Play" on an "Audio Component Instance" (ChasingSoundLoop) while applying a "Volume Curve" (Linear) over a certain time (2 seconds).\nParameters allow designers to indicate the duration of the "Fade" (2 seconds), the "Curve Shape" and the "Start Time" if seeking into the sound.
      (else
        (bind _player_dead_ (CallFunction|IsPlayerDead)) ; Function which checks if the Player is already "dead"!
        (if _player_dead_
          ;;[0.5052 0.5052 0.5052 1 30] "ChasingSoundLoop" Audio Component will Play softer and softer (Linear Fade Curve) over 2 seconds, until stopping completely.
          (Audio|Components|Audio|FadeOut (Variables|Default|GetChasingSoundLoop) 2.0 0.0 "Linear" :!class /Script/Engine.AudioComponent) ; This allows designers to call "Play" on an "Audio Component Instance" (ChasingSoundLoop) while applying a "Volume Curve" (Linear) over a certain time (2 seconds).\nParameters allow designers to indicate the duration of the "Fade" (2 seconds), the "Curve Shape" and the "Start Time" if seeking into the sound.
        )))))

(event Custom|Stop%20Seeing%20And%20Hearing%20Pawn
  ;[1 0.2817 0.1317 0.2 50] EnemyAI will stop seeing and hearing the Player, just 1 second each time it loses track of the Player (All based on "Pawn Sensing Component" AI configuration values), then the EnemyAI will "RoamAround" again.
  ;;[0.2188 0.2188 0.2188] "seeing_or_hearingPlayer?" is a bool variable/key in the "BD_AI" and we'll set it to FALSE
  (AI|Components|Blackboard|SetValueasBool (AI|GetBlackboard (AI|GetAIController self)) (Utilities|Name|MakeLiteralName "seeing_or_hearingPlayer?") false)
  ;[0 1 0.25 0.2 50] After 0.5 seconds Delay, "Chasing_Violins_Loop" Sound will "Fade Out" (2 seconds Duration), if the EnemyAI is not seeing or hearing the Player anymore and "ChasingSoundLoop" Audio Component is Playing at this moment.
  (Utilities|FlowControl|Delay 0.5)
  (if (not (ScalableFloat|GetValueasBool (AI|GetBlackboard (AI|GetAIController self)) (Utilities|Name|MakeLiteralName "seeing_or_hearingPlayer?")))
    (if (Utilities|IsValid (Variables|Default|GetChasingSoundLoop))
      ;;[0.4427 0.4427 0.4427 1 30] "ChasingSoundLoop" Audio Component will Play softer and softer (Linear Fade Curve) over 2 seconds, until it stops completely (Volume = 0)
      (Audio|Components|Audio|FadeOut (Variables|Default|GetChasingSoundLoop) 2.0 0.0 "Linear" :!class /Script/Engine.AudioComponent) ; This allows designer to call a "delayed STOP" (2 seconds) on an "Audio Component Instance" (ChasingSoundLoop) while applying a "Volume Curve" (Linear) over "Fade Out Duration" time.\nParameters allow designers to indicate the duration of the "Fade" (2 seconds) and the "Curve Shape" (Linear).
    )))

(event Custom|AttackPlayer
  (params (Anim%20Montage%20AI :type Anim%20Montage%20Object%20Reference%20%28by%20ref%29) (Anim%20Duration%20AI :type Float%20%28double-precision%29) (Anim%20Apply%20Damage%20AI :type Float%20%28double-precision%29))
  (bind _attack_trace_point (Variables|Default|GetAttack%20Trace%20Point))
  (bind _returnvalue (Transformation|GetWorldLocation _attack_trace_point))
  ;[0 0.1 1 0.2 50] Attack Player Animation Montages (Random Choice between 3 AnimMontages) + Sphere Trace for the Player + Apply Damage (value based on the random AnimMontage that was chosen) to the Player.
  ; The EnemyAI cannot Attack the Player if the EnemyAI is already STUNNED, DEAD or the Player has already DIED.
  (bind _asbp_true_first_person_character (Utilities|Casting|CastToBP_TrueFirstPersonCharacter (Game|GetPlayerCharacter 0)))
  (if (and (and (not (Variables|Default|GetEnemyAI%20attacking?)) (not (Variables|/Game/ThirdPerson/Blueprints/BP_TrueFirstPersonCharacter.BP_TrueFirstPersonCharacter_C|GetPlayer%20attacking? _asbp_true_first_person_character))) (and (not (Variables|/Game/ThirdPerson/Blueprints/BP_TrueFirstPersonCharacter.BP_TrueFirstPersonCharacter_C|GetPlayer%20dead? _asbp_true_first_person_character)) (and (not (Variables|Default|GetEnemyAI%20stunned?)) (not (Variables|Default|GetEnemyAI%20dead?)))))
    (Variables|Default|SetEnemyAI%20attacking? true)
    (Animation|Montage|PlayMontage (Variables|Character|GetMesh) Anim%20Montage%20AI ; Random AnimMontage to Play
      (:then
        (Variables|Default|Setanimation%20Duration Anim%20Duration%20AI)
        (bind (_outhit _returnvalue_2) (Collision|SphereTraceForObjects _returnvalue (+ _returnvalue (* (Math|Vector|GetForwardVector (Transformation|GetWorldRotation _attack_trace_point)) 7e+01)) 25.0 (Utilities|Array|MakeArray "ObjectTypeQuery3") false 0 (Variables|Default|GetDraw%20Debug%20Type))) ; Sweeps a sphere along the given line and returns the first hit encountered. This applies for "AttackTracePoint" Arrow.\nThis sphere only finds objects that are of a type specified by "Object Types"Array (The Arrow will detect types of "Pawn", such as the actual Player)
        (if _returnvalue_2 ; TRUE if there was a hit, FALSE otherwise
          (Game|Damage|ApplyDamage (.HitActor (Collision|BreakHitResult _outhit)) Anim%20Apply%20Damage%20AI 0 0) ; Hurts the player each time with a random damage ('25.0', '30.0' and '35.0')
        ))
      (:OnCompleted
        (Variables|Default|SetEnemyAI%20attacking? false :!label _label))
      (:OnInterrupted
        (goto _label)))))

(event EventBeginPlay
  (Variables|Default|SetEnemyAI%20dead? false :!pinned true) ; EnemyAI is "Alive"!
  ;[1 0.2817 0.1317 0.2 50] EnemyAI will stop seeing and hearing the Player, just 1 second each time it loses track of the Player (All based on "Pawn Sensing Component" AI configuration values), then the EnemyAI will "RoamAround" again.
  (Utilities|Time|SetTimerbyEvent (delegate Custom|Stop%20Seeing%20And%20Hearing%20Pawn) 1.0 true) ; Set a timer (example: 1 second) to execute an Event ("Stop Seeing And Hearing Pawn")
)

(event Collision|EventActorBeginOverlap
  (params (OtherActor :type Actor%20Object%20Reference)))

(event EventTick
  (params (DeltaSeconds :type Float%20%28single-precision%29)))

(event Game|Damage|EventAnyDamage
  (params (Damage :type Float%20%28single-precision%29) (DamageType :type Damage%20Type%20Object%20Reference) (InstigatedBy :type Controller%20Object%20Reference) (DamageCauser :type Actor%20Object%20Reference))
  ;[1 0.25 0 0.25 50] The EnemyAI takes some Damage from the Player (The EnemyAI gets hurt), decreasing EnemyAI's total Health ( + Received Damage Text Animation when Hurt ), then we have 2 cases:
  ;
  ; -> If the EnemyAI's Health stayes above '0.0', the EnemyAI will get STUNNED (being unable to move) until "Zombie_Reaction_Hit_Montage" Montage is COMPLETED or INTERRUPTED [ +  "Monster_Pain_Grunt_1" 3D Sound if the Player is equipped with a Weapon, otherwise "Monster_Pain_Grunt_2" 3D Sound (Both 3D Sounds at EnemyAI Location + "SA_Character" Sound Attenuation) ];
  ;
  ; -> If the EnemyAI's Health reaches '0.0' or below, the EnemyAI will collapse to the floor (being DEAD), stopping the currently Running Brain Logic of the "AIController's" Behavior Tree [ + "Monster_Death_Grunt" 3D Sound (at EnemyAI Location + "SA_Character" Sound Attenuation) ].
  ;      '2.0' seconds after EnemyAI's Death, a SECOND "Objective Notification" will appear on the screen, then a BRIGHT PORTAL will be spawned in the World with the specified "Transform (Location, Rotation, Scale)" Coordinates;
  (Variables|Default|SetCurrent%20Received%20Damage%20Value Damage)
  (Variables|Default|SetEnemyAI%20Health (Math|Float|Clamp(Float) (- (Variables|Default|GetEnemyAI%20Health) Damage) 0.0 1e+02))
  (Variables|Default|GetWB%20Received%20Damage%20Indicator ; "Validated Get" adds in Branching Execution Pins so that we can separately handle when the Returned Value\n("WB_Received_Damage_Indicator" Value) is Valid (Widget already created) or Invalid (Widget not created yet).
    (:then
      _)
    (:else
      (bind _returnvalue (UserInterface|CreateWidget "/Game/UI/WB_Received_Damage_Indicator.WB_Received_Damage_Indicator_C" (Game|GetPlayerController 0))) ; Creates the "WB_Received_Damage_Indicator" Widget
      (bind _output_get (Variables|Default|SetWB%20Received%20Damage%20Indicator _returnvalue))
      (UserInterface|Viewport|AddtoViewport _output_get -10 :!pinned true) ; ZOrder = -10
    ))
  (Default|PlayReceivedDamageAnimation (Variables|Default|GetWB%20Received%20Damage%20Indicator)) ; Custom Event which will Play "ReceivedDamage" Animation\nfrom "WB_Received_Damage_Indicator" Widget
  (if (> (Variables|Default|GetEnemyAI%20Health) 0.0)
    (Variables|Default|SetEnemyAI%20stunned? true)
    (Variables|/Script/Engine.CharacterMovementComponent|SetMaxWalkSpeed (Variables|Character|GetCharacterMovement) 0.0)
    (bind _player_has_weapon_ (CallFunction|DoesPlayerHaveWeapon)) ; Functions which checks if the Player is equipped with a Weapon
    (if _player_has_weapon_
      (Audio|PlaySoundatLocation "/Game/Audio/SFX/Monster_Pain_Grunt_1.Monster_Pain_Grunt_1" (Transformation|GetActorLocation) "0, 0, 0" 1.0 1.0 0.0 "/Game/Audio/SFX/SA_Character.SA_Character" 0 0 0) ; "Monster_Pain_Grunt_1" 3D Sound\n(at EnemyAI Location + "SA_Character" Sound Attenuation)
      (Components|Activation|Activate (Variables|Default|GetNPS_Component_Blood) false) ; Activates the SceneComponent\n("NPS Component Blood" Niagara Particle System)
      (Animation|Montage|PlayMontage (Variables|Character|GetMesh) "/Game/AI/ParasiteAI/Animations/Montages/Zombie_Reaction_Hit_Montage.Zombie_Reaction_Hit_Montage" ; Plays "Zombie_Reaction_Hit_Montage" Montage
        (:OnCompleted
          _)
        (:OnInterrupted
          _))
      (Variables|Default|SetEnemyAI%20stunned? false)
      (Components|Activation|Deactivate (Variables|Default|GetNPS_Component_Blood)) ; Deactivates the SceneComponent\n("NPS Component Blood" Niagara Particle System)
      (else
        (Audio|PlaySoundatLocation "/Game/Audio/SFX/Monster_Pain_Grunt_2.Monster_Pain_Grunt_2" (Transformation|GetActorLocation) "0, 0, 0" 1.0 1.0 0.0 "/Game/Audio/SFX/SA_Character.SA_Character" 0 0 0) ; "Monster_Pain_Grunt_2" 3D Sound\n(at EnemyAI Location + "SA_Character" Sound Attenuation)
        (Animation|Montage|PlayMontage (Variables|Character|GetMesh) "/Game/AI/ParasiteAI/Animations/Montages/Zombie_Reaction_Hit_Montage.Zombie_Reaction_Hit_Montage" ; Plays "Zombie_Reaction_Hit_Montage" Montage
          (:OnCompleted
            _)
          (:OnInterrupted
            _))
        (Variables|Default|SetEnemyAI%20stunned? false)))
    (else
      (Variables|Default|SetEnemyAI%20dead? true :!pinned true) ; EnemyAI "Died"!
      (Audio|PlaySoundatLocation "/Game/Audio/SFX/Monster_Death_Grunt.Monster_Death_Grunt" (Transformation|GetActorLocation) "0, 0, 0" 1.0 1.0 0.0 "/Game/Audio/SFX/SA_Character.SA_Character" 0 0 0) ; "Monster_Death_Grunt" 3D Sound\n(at EnemyAI Location + "SA_Character" Sound Attenuation)
      (Physics|SetSimulatePhysics (Variables|Character|GetMesh) true) ; Sets the "Mesh" Component to use physics simulation\n("Simulate" bool = TRUE), otherwise it will be 'fixed' (kinematic)
      (Pawn|Components|CharacterMovement|SetMovementMode (Variables|Character|GetCharacterMovement) "MOVE_None" 0) ; EnemyAI cannot move anymore\n("New Movement Mode" = None)
      (AI|Logic|StopLogic (Variables|/Script/AIModule.AIController|GetBrainComponent (AI|GetAIController self)) "EnemyAI is DEAD!") ; Stops currently Running Brain Logic of\nthe "AIController's" Behavior Tree
      ;;[1 0.25 0.75 0.2 40] "Objective Index" Variable from Player's Blueprint will be "Incremented" just after a '1.5' seconds Delay, the SECOND Objective Notification appearing on the screen after another '0.5' seconds Delay -> Total '2.0' seconds Delay ( + "NewObjective_Notification" 2D Sound ).
      (bind _asbp_true_first_person_character (Utilities|Casting|CastToBP_TrueFirstPersonCharacter (Game|GetPlayerCharacter 0)))
      (Utilities|FlowControl|Delay 1.5) ; '1.5' seconds Delay
      (Math|Integer|IncrementInt (Variables|/Game/ThirdPerson/Blueprints/BP_TrueFirstPersonCharacter.BP_TrueFirstPersonCharacter_C|GetObjective%20Index _asbp_true_first_person_character) ; Adds '1' to the specified value then sets it\n("++ObjectiveIndex" in CPP)
        (:%20%20
          (Utilities|FlowControl|Delay 0.5) ; '0.5' seconds Delay
          (Audio|PlaySound2D "/Game/Audio/SFX/NewObjective_Notification.NewObjective_Notification" 1.0 1.0 0.0 0 0) ; "NewObjective_Notification" 2D Sound
          (Default|PlayNewObjectiveAnimation (Variables|/Game/ThirdPerson/Blueprints/BP_TrueFirstPersonCharacter.BP_TrueFirstPersonCharacter_C|GetWB%20Objectives _asbp_true_first_person_character)) ; Custom Event which will Play "NewObjective"\nAnimation from "WB_Objectives" Widget
          ;;[0 0.5 0.5 0.2 40] Spawning the "Portal" Actor ("BP_Portal") in the World with the EXACT corresponding "Transform" Coordinates [ Location  = (10360, 51110, 1930), Rotation = (0, 0, 0), Scale = (15, 15, 15) ], "Ignoring Collisions", Player being the "Instigator" Pawn.
          (bind _asbp_true_first_person_character_2 (Utilities|Casting|CastToBP_TrueFirstPersonCharacter (Game|GetPlayerCharacter 0)))
          (Game|SpawnActorfromClass "/Game/Blueprints/BP_Portal.BP_Portal_C" (Math|Transform|MakeTransform "10360.000000,51110.000000,1930.000000" "0, 0, 0" "15.000000,15.000000,15.000000") "AlwaysSpawn" "OverrideRootScale" 0 _asbp_true_first_person_character_2) ; Always Spawns the "Portal" Actor with the specified "Transform (Location, Rotation, Scale)",\n"Ignoring Collisions" and using the exact "Transform Scale" Coordinates set in the "BP_Portal".\nPlayer is the "Instigator" Pawn responsible for damage and other gameplay events caused by "BP_Portal" Actor.
        )))))

(fn ConstructionScript)

(fn GetARandomAnimAttack
  (bind _anim_attacks (Variables|Default|GetAnim%20Attacks))
  (bind _returnvalue (Utilities|Array|Length _anim_attacks))
  (bind _returnvalue_2 (- _returnvalue 1))
  (bind _returnvalue_3 (Math|Random|RandomIntegerinRange 0 _returnvalue_2))
  (bind _output (Utilities|Array|Get(acopy) _anim_attacks _returnvalue_3))
  (bind (_animmontageai _animdurationai _animapplydamageai) (Utilities|Struct|BreakAnimAttackStruct _output))
  ;[0.4419 0.4222 1 0.2 40] Function which will choose a Random AnimMontage and its corresponding Duration from the Array of Structure "AnimMontage_AnimDuration".
  (return _animmontageai _animdurationai _animapplydamageai))

(fn IsPlayerDead
  ;[1 0.7178 0.3816 0.2 40] Returns TRUE if the Player is already "dead", otherwise FALSE.
  (bind _asbp_true_first_person_character (Utilities|Casting|CastToBP_TrueFirstPersonCharacter (Game|GetPlayerCharacter 0)))
  (return (Variables|/Game/ThirdPerson/Blueprints/BP_TrueFirstPersonCharacter.BP_TrueFirstPersonCharacter_C|GetPlayer%20dead? _asbp_true_first_person_character)))

(fn DoesPlayerHaveWeapon
  ;[1 0.25 0 0.2 40] Returns TRUE if the Player is already equipped with a Weapon, otherwise FALSE.
  (bind _asbp_true_first_person_character (Utilities|Casting|CastToBP_TrueFirstPersonCharacter (Game|GetPlayerCharacter 0)))
  (return (Variables|/Game/ThirdPerson/Blueprints/BP_TrueFirstPersonCharacter.BP_TrueFirstPersonCharacter_C|GetPlayer%20has%20Axe%20Weapon? _asbp_true_first_person_character)))