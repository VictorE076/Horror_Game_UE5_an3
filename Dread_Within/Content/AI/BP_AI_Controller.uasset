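; AI controller for the enemy character that runs the BT_AI behavior tree and reacts to heard noises.
; Perception updates from a BP_HidingPlace store the door noise location and set the "door_noise_heard?" blackboard flag.
; Every perception update writes LastNoiseHeardLocation on the BP_EnemyAI found by GetActorOfClass, rather than on the controlled pawn.
; The Died event detaches the pawn from the controller pending destroy.
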(event OnTargetPerceptionUpdated(AIPerception)
  (params (Actor :type Actor%20Object%20Reference) (Stimulus :type AI%20Stimulus%20Structure))
  (bind _stimuluslocation (Utilities|Struct|BreakAIStimulus Stimulus))
  ;[0 0 1 0.2 50] Event triggered only when EnemyAI senses noise from one HidingPlace.
  ;
  ; UPDATE   ->   "LastNoiseHeardLocation" each time EnemyAI hears any noise (from HidingPlace's Door + the Player's Footsteps).
  (Utilities|Casting|CastToBP_HidingPlace Actor
    (:then
      (Variables|AIPerception|SetDoorNoiseLocation _stimuluslocation)
      ;;[0.4896 0.4896 0.4896 1 30] "door_noise_heard?" is a bool variable/key in the "BD_AI" and we'll set it to TRUE
      (AI|Components|Blackboard|SetValueasBool (Variables|Default|GetBlackboard) (Utilities|Name|MakeLiteralName "door_noise_heard?") true)
      (Development|PrintString "Door Noise" true true "(R=1.000000,G=0.700000,B=0.000000,A=1.000000)" 5.0))
    (:CastFailed
      _))
  ;;[0.3 0.3 0.1 0.5 30] Last Noise Heard Location
  (bind _returnvalue (Actor|GetActorOfClass "/Game/AI/BP_EnemyAI.BP_EnemyAI_C"))
  (Utilities|IsValid _returnvalue
    (:Is%20Valid
      (bind _output_get (Variables|/Game/AI/BP_EnemyAI.BP_EnemyAI_C|SetLastNoiseHeardLocation _returnvalue _stimuluslocation))
      (Development|PrintString (Utilities|String|ToString(Vector) _output_get) false false "(R=0.000000,G=1.000000,B=1.000000,A=1.000000)" 5.0))))

(event Custom|Died
  ;[0 0.5 1 0.2 50] "BT_AI" Behavior Tree becomes INACTIVE
  (Class|Pawn|DetachfromControllerPendingDestroy (Pawn|GetControlledPawn)) ; Detaching the EnemyAI from its AI_Controller
)

(event EventBeginPlay
  ;[0.5 0 1 0.2 50] "BT_AI" Behavior Tree
  (AI|RunBehaviorTree "/Game/AI/BT_AI.BT_AI" :!pinned true) ; Starts executing "Behavior Tree"
)

(event EventTick
  (params (DeltaSeconds :type Float%20%28single-precision%29)))

(fn ConstructionScript)