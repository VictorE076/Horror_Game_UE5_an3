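; Hiding place actor with a swinging door that the player toggles through Interact.
; Interact plays a squeak, reports an AI noise event and rotates the door with open or close timelines, using a flag on the player to block moves mid-swing.
; Inside and outside triggers manage the player's door prompt, clearing it only when neither overlaps.
; The inside trigger also records on the player whether they are hiding and this place's world ID.
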(event OnComponentBeginOverlap(TriggerInside)
  (params (OverlappedComponent :type Primitive%20Component%20Object%20Reference) (OtherActor :type Actor%20Object%20Reference) (OtherComp :type Primitive%20Component%20Object%20Reference) (OtherBodyIndex :type Integer) (bFromSweep :type Boolean) (SweepResult :type Hit%20Result%20Structure%20%28by%20ref%29))
  ;[1 0.25 0 0.2 50] "Player Inside An Hiding Place?" bool variable is set to TRUE (from Player's Blueprint) AND "Hiding Place ID World" (from Player's Blueprint) is set to the corresponding "ID World" Value, when Player starts to overlap the "TriggerInside" Component. The "WB_Interaction Message" Variable from Player's Blueprint will change to "Press 'R' to open/close the door!"
  (bind _asbp_true_first_person_character (Utilities|Casting|CastToBP_TrueFirstPersonCharacter OtherActor))
  (Variables|/Game/ThirdPerson/Blueprints/BP_TrueFirstPersonCharacter.BP_TrueFirstPersonCharacter_C|SetPlayer%20Inside%20An%20HidingPlace? _asbp_true_first_person_character true)
  (bind _output_get (Variables|/Game/ThirdPerson/Blueprints/BP_TrueFirstPersonCharacter.BP_TrueFirstPersonCharacter_C|SetHidingPlace%20ID%20World _asbp_true_first_person_character (Variables|Default|GetID%20World)))
  (Development|PrintString (Utilities|String|ToString(Integer) _output_get))
  (Variables|/Game/ThirdPerson/Blueprints/BP_TrueFirstPersonCharacter.BP_TrueFirstPersonCharacter_C|SetWB_Interaction%20Message _asbp_true_first_person_character "Press 'R' to open/close the door!")
  (Development|PrintString "Inside" false false "(R=0.000000,G=0.500000,B=0.000000,A=1.000000)" 5.0))

(event OnComponentEndOverlap(TriggerInside)
  (params (OverlappedComponent :type Primitive%20Component%20Object%20Reference) (OtherActor :type Actor%20Object%20Reference) (OtherComp :type Primitive%20Component%20Object%20Reference) (OtherBodyIndex :type Integer))
  ;[1 0.25 0 0.2 50] "Player Inside An Hiding Place?" bool variable is set to FALSE (from Player's Blueprint) AND "Hiding Place ID World" (from Player's Blueprint) is reset to '-1', when Player stops overlapping the "TriggerInside" Component. The "WB_Interaction Message" Variable from Player's Blueprint will be empty (If Player is not currently overlapping "TriggerOutside" Component).
  (bind _asbp_true_first_person_character (Utilities|Casting|CastToBP_TrueFirstPersonCharacter OtherActor))
  (Variables|/Game/ThirdPerson/Blueprints/BP_TrueFirstPersonCharacter.BP_TrueFirstPersonCharacter_C|SetPlayer%20Inside%20An%20HidingPlace? _asbp_true_first_person_character false)
  (bind _output_get (Variables|/Game/ThirdPerson/Blueprints/BP_TrueFirstPersonCharacter.BP_TrueFirstPersonCharacter_C|SetHidingPlace%20ID%20World _asbp_true_first_person_character -1))
  (Development|PrintString (Utilities|String|ToString(Integer) _output_get))
  (if (not (Collision|IsOverlappingActor (Variables|Default|GetTriggerOutside) OtherActor :!class /Script/Engine.PrimitiveComponent))
    (Variables|/Game/ThirdPerson/Blueprints/BP_TrueFirstPersonCharacter.BP_TrueFirstPersonCharacter_C|SetWB_Interaction%20Message _asbp_true_first_person_character "")
    (Development|PrintString "Inside" false false "(R=0.500000,G=0.000000,B=0.000000,A=1.000000)" 5.0)))

(event OnComponentBeginOverlap(TriggerOutside)
  (params (OverlappedComponent :type Primitive%20Component%20Object%20Reference) (OtherActor :type Actor%20Object%20Reference) (OtherComp :type Primitive%20Component%20Object%20Reference) (OtherBodyIndex :type Integer) (bFromSweep :type Boolean) (SweepResult :type Hit%20Result%20Structure%20%28by%20ref%29))
  ;[1 0.5 0 0.2 50] When the Player starts to overlap the "TriggerOutside" Component, it will set the "WB_Interaction Message" Variable from Player's Blueprint to "Press 'R' to open/close the door!", then when the Player stops overlapping the same Component, the respective Variable will become empty (If Player is not currently overlapping "TriggerInside" Component).
  (bind _asbp_true_first_person_character (Utilities|Casting|CastToBP_TrueFirstPersonCharacter OtherActor))
  (Variables|/Game/ThirdPerson/Blueprints/BP_TrueFirstPersonCharacter.BP_TrueFirstPersonCharacter_C|SetWB_Interaction%20Message _asbp_true_first_person_character "Press 'R' to open/close the door!")
  (Development|PrintString "Outside" false false "(R=0.000000,G=0.500000,B=0.000000,A=1.000000)" 5.0))

(event OnComponentEndOverlap(TriggerOutside)
  (params (OverlappedComponent :type Primitive%20Component%20Object%20Reference) (OtherActor :type Actor%20Object%20Reference) (OtherComp :type Primitive%20Component%20Object%20Reference) (OtherBodyIndex :type Integer))
  ;[1 0.5 0 0.2 50] When the Player starts to overlap the "TriggerOutside" Component, it will set the "WB_Interaction Message" Variable from Player's Blueprint to "Press 'R' to open/close the door!", then when the Player stops overlapping the same Component, the respective Variable will become empty (If Player is not currently overlapping "TriggerInside" Component).
  (bind _asbp_true_first_person_character (Utilities|Casting|CastToBP_TrueFirstPersonCharacter OtherActor))
  (if (not (Collision|IsOverlappingActor (Variables|Default|GetTriggerInside) OtherActor :!class /Script/Engine.PrimitiveComponent))
    (Variables|/Game/ThirdPerson/Blueprints/BP_TrueFirstPersonCharacter.BP_TrueFirstPersonCharacter_C|SetWB_Interaction%20Message _asbp_true_first_person_character "")
    (Development|PrintString "Outside" false false "(R=0.500000,G=0.000000,B=0.000000,A=1.000000)" 5.0)))

(event Custom|Open%20or%20Close%20Door
  ;[0 0.5 1 0.2 50] ''Event Interact" triggeres the "Open OR Close Door" Custom Event, which will Open/Close the Door of the "BP_HidingPlace" (Added 2 Sounds for Opening/Closing Door + Making/Reporting that squeak noise) by rotating it on ZAxis, between a certain Angle (0.0 - 115.0) and by using 2 "Timeline" Nodes for keyframing a certain value used for the Angle, over a period of Time.
  (bind _asbp_true_first_person_character (Utilities|Casting|CastToBP_TrueFirstPersonCharacter (Game|GetPlayerCharacter 0)))
  (if (Variables|/Game/ThirdPerson/Blueprints/BP_TrueFirstPersonCharacter.BP_TrueFirstPersonCharacter_C|Getcan%20move%20any%20HidingPlace%20Door? _asbp_true_first_person_character)
    (Variables|/Game/ThirdPerson/Blueprints/BP_TrueFirstPersonCharacter.BP_TrueFirstPersonCharacter_C|Setcan%20move%20any%20HidingPlace%20Door? _asbp_true_first_person_character false)
    ;;[0.5 0.5 0.2 0.5 30] "Door" Noise
    (Class|AISenseHearing|ReportNoiseEvent (Transformation|GetWorldLocation (Variables|Default|GetRef_DoorNoise)) 1.0 self 0.0 "None") ; This HidingPlace Instigator reports\n"Door" Noise to AISense
    (if (<= (Variables|Default|GetDoor%20Angle) 0.0)
      (Audio|PlaySoundatLocation "/Game/Audio/SFX/Open_Door_squeak.Open_Door_squeak" (Transformation|GetWorldLocation (Variables|Default|GetDoor)) "0, 0, 0" 1.0 1.0 0.0 0 0 0 0) ; "Open_Door_squeak" Sound at Door's Location
      ;;[0.5 0.5 0.5 1 30] OPEN Door
      (bind _doorzaxisrotation (Timeline|OpenDoor%20Timeline PlayFromStart) ; "Door ZAxis Rotation" value will grow between\n'0' and '1' during '1.1' seconds (time period)
        (:Update
          (Transformation|SetRelativeRotation (Variables|Default|GetDoor) (Math|Rotator|MakeRotator 0.0 0.0 (Math|Float|Lerp 0.0 115.0 _doorzaxisrotation)) false false) ; Set the rotation of the "Door" (Static Mesh Component)\nrelative to Z Axis (between 0 and 115)
        )
        (:Finished
          (Variables|Default|SetDoor%20Angle 115.0)
          (Variables|/Game/ThirdPerson/Blueprints/BP_TrueFirstPersonCharacter.BP_TrueFirstPersonCharacter_C|Setcan%20move%20any%20HidingPlace%20Door? _asbp_true_first_person_character true)))
      (else
        (Audio|PlaySoundatLocation "/Game/Audio/SFX/Close_Door_squeak.Close_Door_squeak" (Transformation|GetWorldLocation (Variables|Default|GetDoor)) "0, 0, 0" 1.0 1.0 0.0 0 0 0 0) ; "Close_Door_squeak" Sound at Door's Location
        ;;[0.5 0.5 0.5 1 30] CLOSE Door
        (bind _doorzaxisrotation_2 (Timeline|CloseDoor%20Timeline ReverseFromEnd) ; "Door ZAxis Rotation" value will shrink between\n'0' and '1' during '0.7' seconds (time period)
          (:Update
            (Transformation|SetRelativeRotation (Variables|Default|GetDoor) (Math|Rotator|MakeRotator 0.0 0.0 (Math|Float|Lerp 0.0 115.0 _doorzaxisrotation_2)) false false) ; Set the rotation of the "Door" (Static Mesh Component)\nrelative to Z Axis (between 0 and 115)
          )
          (:Finished
            (Variables|Default|SetDoor%20Angle 0.0)
            (Variables|/Game/ThirdPerson/Blueprints/BP_TrueFirstPersonCharacter.BP_TrueFirstPersonCharacter_C|Setcan%20move%20any%20HidingPlace%20Door? _asbp_true_first_person_character true)))))))

(event EventBeginPlay)

(event Collision|EventActorBeginOverlap
  (params (OtherActor :type Actor%20Object%20Reference)))

(event EventInteract
  ;[0 0.5 1 0.2 50] ''Event Interact" triggeres the "Open OR Close Door" Custom Event, which will Open/Close the Door of the "BP_HidingPlace" (Added 2 Sounds for Opening/Closing Door + Making/Reporting that squeak noise) by rotating it on ZAxis, between a certain Angle (0.0 - 115.0) and by using 2 "Timeline" Nodes for keyframing a certain value used for the Angle, over a period of Time.
  (CallFunction|OpenorCloseDoor) ; Custom Event triggered for Opening or Closing the Door
)

(fn ConstructionScript)