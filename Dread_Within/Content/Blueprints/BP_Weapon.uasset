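; BP_Weapon is an axe pickup that the first-person player can take.
; Its Trigger overlap events filter by the "Player" tag, toggle AxeOverlapped, and set or clear the "Press 'R'" prompt text on BP_TrueFirstPersonCharacter.
; The Interact event casts the player character and calls its EquipAxeWeapon event, without checking overlap state itself.
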(event OnComponentBeginOverlap(Trigger)
  (params (OverlappedComponent :type Primitive%20Component%20Object%20Reference) (OtherActor :type Actor%20Object%20Reference) (OtherComp :type Primitive%20Component%20Object%20Reference) (OtherBodyIndex :type Integer) (bFromSweep :type Boolean) (SweepResult :type Hit%20Result%20Structure%20%28by%20ref%29))
  ;[0.5 0.25 0 0.2 50] When the Player starts to overlap the "Trigger" Component, it will set the "WB_Interaction Message" Variable from Player's Blueprint to "Press 'R' to take the weapon!" [ if the Player is not already equipped with an Axe Weapon ( Variable "Empty" otherwise ) ], then when the Player stops overlapping the same Component, the respective Variable will become "Empty".
  (if (Actor|ActorHasTag OtherActor "Player")
    (Variables|Weapon|SetAxe%20Overlapped? true)
    (bind _asbp_true_first_person_character (Utilities|Casting|CastToBP_TrueFirstPersonCharacter (Game|GetPlayerCharacter 0)))
    (Variables|/Game/ThirdPerson/Blueprints/BP_TrueFirstPersonCharacter.BP_TrueFirstPersonCharacter_C|SetWB_Interaction%20Message _asbp_true_first_person_character "Press 'R' to take the Axe!")))

(event OnComponentEndOverlap(Trigger)
  (params (OverlappedComponent :type Primitive%20Component%20Object%20Reference) (OtherActor :type Actor%20Object%20Reference) (OtherComp :type Primitive%20Component%20Object%20Reference) (OtherBodyIndex :type Integer))
  ;[0.5 0.25 0 0.2 50] When the Player starts to overlap the "Trigger" Component, it will set the "WB_Interaction Message" Variable from Player's Blueprint to "Press 'R' to take the weapon!" [ if the Player is not already equipped with an Axe Weapon ( Variable "Empty" otherwise ) ], then when the Player stops overlapping the same Component, the respective Variable will become "Empty".
  (if (Actor|ActorHasTag OtherActor "Player")
    (Variables|Weapon|SetAxe%20Overlapped? false)
    (bind _asbp_true_first_person_character (Utilities|Casting|CastToBP_TrueFirstPersonCharacter (Game|GetPlayerCharacter 0)))
    (Variables|/Game/ThirdPerson/Blueprints/BP_TrueFirstPersonCharacter.BP_TrueFirstPersonCharacter_C|SetWB_Interaction%20Message _asbp_true_first_person_character "")))

(event EventBeginPlay)

(event Collision|EventActorBeginOverlap
  (params (OtherActor :type Actor%20Object%20Reference)))

(event EventTick
  (params (DeltaSeconds :type Float%20%28single-precision%29)))

(event EventInteract
  ;[1 0.1892 0.03929 0.2 50] ''Event Interact" equips the Player with an "Axe Weapon".
  (bind _asbp_true_first_person_character (Utilities|Casting|CastToBP_TrueFirstPersonCharacter (Game|GetPlayerCharacter 0)))
  (Default|EquipAxeWeapon _asbp_true_first_person_character) ; Custom Event from "BP_TrueFirstPersonCharacter" (the Player)
)

(fn ConstructionScript)